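; BP_Enemy is an enemy Blueprint with hit points that dies when damage depletes them.
; The Damage event subtracts from HP and prints the remainder, or calls Death when HP would reach zero or below.
; Death grants a fixed Bless amount to the player's 2DSideScrollerCharacter via AddBless, then destroys the enemy.
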(event `Damage`
  (params (Value :type "Float (double-precision)"))
  (bind _returnvalue (- (`self.HP`) Value))
  (if (<= _returnvalue 0.0)
    (`self.Death`)
    (else
      (bind _output_get (set `self.HP` _returnvalue))
      (`KismetSystemLibrary.PrintString` (`KismetStringLibrary.Conv_DoubleToString` _output_get)))))

(event `Death`
  (bind _as2dside_scroller_character (cast `/Game/2DSideScrollerBP/Blueprints/2DSideScrollerCharacter` (`GameplayStatics.GetPlayerPawn` 0)))
  (`/Game/2DSideScrollerBP/Blueprints/2DSideScrollerCharacter.Add Bless` _as2dside_scroller_character 20.0)
  (`self.K2_DestroyActor`))

(fn `UserConstructionScript`)